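; BP_SphereThing is an actor that arranges BP_SphereThingChild actors in a ring or arc around its Cube component.
; AddCube and RemoveCube events grow or shrink the Cubes array, which acts as the child count, then call SpawnSpheres.
; SpawnSpheres destroys all existing children, respawns and attaches them, then spaces them evenly in XY using sine and cosine of Radius and Degrees.
; The construction script and DoMath are empty.
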(event `AddCube`
  (`KismetArrayLibrary.Array_Add` (`self.Cubes`))
  (`self.SpawnSpheres`))

(event `RemoveCube`
  (bind _cubes (`self.Cubes`))
  (if (`KismetArrayLibrary.Array_IsNotEmpty` _cubes)
    (`KismetArrayLibrary.Array_Remove` _cubes)
    (`self.SpawnSpheres`)))

(fn `DoMath`)

(fn `SpawnSpheres`
  (bind _cubes (`self.Cubes`))
  (bind _radius (`self.Radius`))
  (for _array_element (`self.CubeChildren`)
    (`self.K2_DestroyActor` _array_element))
  (`KismetArrayLibrary.Array_Clear` (`self.CubeChildren`))
  (if (`KismetArrayLibrary.Array_IsNotEmpty` _cubes)
    (for (_ _array_index) _cubes
      (bind _returnvalue (`|SpawnActorFromClass` "/Game/Blueprints/BP_SphereThingChild.BP_SphereThingChild_C" (`KismetMathLibrary.MakeTransform` (0.0 0.0 0.0)) "Undefined" "MultiplyWithRoot" null null))
      (`KismetArrayLibrary.Array_Add` (`self.CubeChildren`) _returnvalue)
      (`self.K2_AttachToComponent` _returnvalue (`self.Cube`) "None" "SnapToTarget" "KeepRelative" "KeepWorld" true)
      (bind _returnvalue_2 (* _array_index (/ (`self.Degrees`) (`KismetMathLibrary.Conv_IntToDouble` (`KismetArrayLibrary.Array_Length` _cubes)))))
      (`self.K2_SetActorRelativeLocation` _returnvalue (`KismetMathLibrary.MakeVector` (* _radius (`KismetMathLibrary.DegCos` _returnvalue_2)) (* _radius (`KismetMathLibrary.DegSin` _returnvalue_2))) false false))))

(fn `UserConstructionScript`)