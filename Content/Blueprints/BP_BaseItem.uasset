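; BP_BaseItem is a holdable grapple gun item with use, alternate use and drop events.
; Use and AltUse call Grapple and AltGrapple on the player's first-person character and play a shoot sound.
; Drop applies a forward force and re-enables the gun's collision and physics.
; Pickup only returns an enum value; the logic attaching the gun to the character's HoldPoint is disconnected.
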(event `self.Use`
  (bind _asbp_first_person_character (cast `/Game/FirstPerson/Blueprints/BP_FirstPersonCharacter` (`GameplayStatics.GetPlayerCharacter` 0)))
  (`/Game/FirstPerson/Blueprints/BP_FirstPersonCharacter.Grapple` _asbp_first_person_character)
  (`GameplayStatics.PlaySound2D` "/Game/FirstPerson/shoot.shoot" 1.0 1.0 0.0 null null))

(event `self.AltUse`
  (bind _asbp_first_person_character (cast `/Game/FirstPerson/Blueprints/BP_FirstPersonCharacter` (`GameplayStatics.GetPlayerCharacter` 0)))
  (`/Game/FirstPerson/Blueprints/BP_FirstPersonCharacter.AltGrapple` _asbp_first_person_character)
  (`GameplayStatics.PlaySound2D` "/Game/FirstPerson/shoot.shoot" 1.0 1.0 0.0 null null))

(event `self.Drop`
  (bind _grapplegun (`self.GrappleGun`))
  (`PhysicsThreadLibrary.AddForce` (struct) (* (`SceneComponent.GetForwardVector` _grapplegun) 20000.0))
  (`PrimitiveComponent.SetCollisionEnabled` _grapplegun "QueryAndPhysics")
  (`PrimitiveComponent.SetSimulatePhysics` (`self.GrappleGun`) true))

(fn `Pickup`
  (params (Owner :type "/Game/Blueprints/BPC_Interact Object Reference"))
  (returns (ItemType :type "/Game/Blueprints/ENUM_Items Enum"))
  (return "NewEnumerator11"))

(fn `UserConstructionScript`)