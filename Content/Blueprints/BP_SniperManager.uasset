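; Sniper manager actor that starts recurring sniper activations when the player enters its trigger box.
; Overlap by the first person character calls ActivateSniper, which activates a random entry from the Snipers array.
; ActivateSniper then waits six seconds and calls itself, looping indefinitely with no stop condition or guard against repeated overlaps.
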(event `ActivateSniper`
  (bind _snipers (`self.Snipers`))
  (`/Game/Blueprints/BP_SniperSpot.Activate` (`|GetArrayItem` _snipers (`KismetMathLibrary.RandomIntegerInRange` 0 (- (`KismetArrayLibrary.Array_Length` _snipers) 1))))
  (`KismetSystemLibrary.Delay` 6.0)
  (`self.ActivateSniper`))

(event `self.Box.OnComponentBeginOverlap`
  (params (OverlappedComponent :type "PrimitiveComponent Object Reference") (OtherActor :type "Actor Object Reference") (OtherComp :type "PrimitiveComponent Object Reference") (OtherBodyIndex :type Integer) (bFromSweep :type Boolean) (SweepResult :type "HitResult Structure (by ref)"))
  (cast `/Game/FirstPerson/Blueprints/BP_FirstPersonCharacter` OtherActor)
  (`self.ActivateSniper`))

(fn `UserConstructionScript`)