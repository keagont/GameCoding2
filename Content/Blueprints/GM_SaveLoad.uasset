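; Game mode that saves and loads the player's inventories, location and level stage.
; Player data (belt and backpack) uses one slot, while level state uses a slot suffixed with the level name.
; BeginPlay creates missing save objects, then calls Load to activate level actors and restore inventories and player transform.
; With an existing player save, BeginPlay also reapplies inventories after a short delay.
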(event `self.ReceiveBeginPlay`
  (bind _playersave (`self.PlayerSave`))
  (`|ExecutionSequence`
    (:`then_0`
      (bind _returnvalue (`GameplayStatics.DoesSaveGameExist` (`self.SlotName`)))
      (if _returnvalue
        (`KismetSystemLibrary.Delay` 0.2)
        (bind _asbp_first_person_character (cast `/Game/FirstPerson/Blueprints/BP_FirstPersonCharacter` (`GameplayStatics.GetPlayerCharacter` 0)))
        (bind _bpc_invbelt (`/Game/FirstPerson/Blueprints/BP_FirstPersonCharacter.BPC_InvBelt` _asbp_first_person_character))
        (bind _output_get (set `/Game/Blueprints/BPC_Inventory.EnumInventory` (`/Game/Blueprints/SG_Player.Belt` _playersave) _bpc_invbelt))
        (`/Game/Blueprints/BPC_Inventory.SetEnumArray` _bpc_invbelt _output_get)
        (bind _bpc_invbackpack (`/Game/FirstPerson/Blueprints/BP_FirstPersonCharacter.BPC_InvBackPack` _asbp_first_person_character))
        (bind _output_get_2 (set `/Game/Blueprints/BPC_Inventory.EnumInventory` (`/Game/Blueprints/SG_Player.Inv` _playersave) _bpc_invbackpack))
        (`/Game/Blueprints/BPC_Inventory.SetEnumArray` _bpc_invbackpack _output_get_2)
        (else
          (`self.CreatePlayerSave`))))
    (:`then_1`
      (bind _returnvalue_2 (`GameplayStatics.GetCurrentLevelName` true))
      (bind _returnvalue_3 (`GameplayStatics.DoesSaveGameExist` (`KismetStringLibrary.Concat_StrStr` (`self.SlotName`) "_" _returnvalue_2)))
      (if (not _returnvalue_3)
        (`self.CreateLevelSave`)))
    (:`then_2`
      (`KismetSystemLibrary.Delay` 0.0)
      (`self.Load`))))

(fn `CreateLevelSave`
  (bind _returnvalue (`GameplayStatics.CreateSaveGameObject` "/Game/Blueprints/SG_LevelState.SG_LevelState_C"))
  (set `self.LevelState` _returnvalue))

(fn `CreatePlayerSave`
  (bind _returnvalue (`GameplayStatics.CreateSaveGameObject` "/Game/Blueprints/SG_Player.SG_Player_C"))
  (set `self.PlayerSave` _returnvalue))

(fn `Load`
  (bind _playersave (`self.PlayerSave`))
  (bind _returnvalue (`GameplayStatics.LoadGameFromSlot` (`self.SlotName`)))
  (bind _assg_player (cast `/Game/Blueprints/SG_Player` _returnvalue))
  (set `self.PlayerSave` _assg_player)
  (bind _returnvalue_2 (`GameplayStatics.GetCurrentLevelName` true))
  (bind _returnvalue_3 (`GameplayStatics.LoadGameFromSlot` (`KismetStringLibrary.Concat_StrStr` (`self.SlotName`) "_" _returnvalue_2)))
  (bind _assg_level_state (cast `/Game/Blueprints/SG_LevelState` _returnvalue_3))
  (bind _output_get (set `self.LevelState` _assg_level_state))
  (`/Game/Blueprints/SG_LevelState.ActivateActors` _output_get)
  (bind _asbp_first_person_character (cast `/Game/FirstPerson/Blueprints/BP_FirstPersonCharacter` (`GameplayStatics.GetPlayerCharacter` 0)))
  (bind _bpc_invbelt (`/Game/FirstPerson/Blueprints/BP_FirstPersonCharacter.BPC_InvBelt` _asbp_first_person_character))
  (bind _output_get_2 (set `/Game/Blueprints/BPC_Inventory.EnumInventory` (`/Game/Blueprints/SG_Player.Belt` _playersave) _bpc_invbelt))
  (`/Game/Blueprints/BPC_Inventory.SetEnumArray` _bpc_invbelt _output_get_2)
  (bind _bpc_invbackpack (`/Game/FirstPerson/Blueprints/BP_FirstPersonCharacter.BPC_InvBackPack` _asbp_first_person_character))
  (bind _output_get_3 (set `/Game/Blueprints/BPC_Inventory.EnumInventory` (`/Game/Blueprints/SG_Player.Inv` _playersave) _bpc_invbackpack))
  (`/Game/Blueprints/BPC_Inventory.SetEnumArray` _bpc_invbackpack _output_get_3)
  (`/Game/FirstPerson/Blueprints/BP_FirstPersonCharacter.LoadTransform` _asbp_first_person_character (`/Game/Blueprints/SG_LevelState.PlayerSavedLocation` (`self.LevelState`))))

(fn `Save`
  (params (Belt :type "Array of /Game/Blueprints/ENUM_Items Enum") (Inv :type "Array of /Game/Blueprints/ENUM_Items Enum") (PlayerSavedLocation :type "Transform Structure") (Stage :type Integer))
  (bind _playersave (`self.PlayerSave`))
  (bind _levelstate (`self.LevelState`))
  (`|ExecutionSequence`
    (:`then_0`
      (set `/Game/Blueprints/SG_Player.Belt` Belt _playersave)
      (set `/Game/Blueprints/SG_Player.Inv` Inv _playersave)
      (`GameplayStatics.SaveGameToSlot` (`self.PlayerSave`) (`self.SlotName`)))
    (:`then_1`
      (bind _output_get (set `/Game/Blueprints/SG_LevelState.PlayerSavedLocation` PlayerSavedLocation _levelstate))
      (set `/Game/Blueprints/SG_LevelState.Stage` Stage _levelstate)
      (`KismetSystemLibrary.PrintText` (`|FormatText` "saving player location at {x}, {y}, {z}" (.x (.location _output_get)) (.y (.location _output_get)) (.z (.location _output_get))))
      (bind _returnvalue (`GameplayStatics.GetCurrentLevelName` true))
      (`GameplayStatics.SaveGameToSlot` (`self.LevelState`) (`KismetStringLibrary.Concat_StrStr` (`self.SlotName`) "_" _returnvalue)))))

(fn `UserConstructionScript`)