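; Sniper spot that, when activated, aims a visible Cable line at the player and fires after a three-second warning.
; Activate shows the cable and starts Track, which re-traces toward the player on a short delay loop and moves the cable's end to the impact point.
; Shoot runs a final trace and restarts the level if it hits BP_FirstPersonCharacter, then the spot deactivates.
; Both traces draw debug lines, and tracking prints the hit actor's name.
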(event `Shoot`
  (bind _outhit (`KismetSystemLibrary.LineTraceSingle` :`Start` (`SceneComponent.K2_GetComponentLocation` (`self.Cable`)) :`End` (`self.K2_GetActorLocation` (`GameplayStatics.GetPlayerCharacter` 0)) :`TraceChannel` "TraceTypeQuery2" :`bTraceComplex` true :`DrawDebugType` "ForDuration" :`DrawTime` 0.1))
  (bind _asbp_first_person_character (cast `/Game/FirstPerson/Blueprints/BP_FirstPersonCharacter` (`.HitActor` (`GameplayStatics.BreakHitResult` _outhit))))
  (`/Game/FirstPerson/Blueprints/BP_FirstPersonCharacter.RestartLevel` _asbp_first_person_character))

(event `Deactivate`
  (`SceneComponent.SetVisibility` (`self.Cable`) false false)
  (set `self.Active` false))

(event `Activate`
  (`SceneComponent.SetVisibility` (`self.Cable`) true false)
  (set `self.Active` true)
  (`self.Track`)
  (`KismetSystemLibrary.Delay` 3.0)
  (`self.Shoot`)
  (`self.Deactivate`))

(event `Track`
  (if (`self.Active`)
    (bind _outhit (`KismetSystemLibrary.LineTraceSingle` :`Start` (`SceneComponent.K2_GetComponentLocation` (`self.Cable`)) :`End` (`self.K2_GetActorLocation` (`GameplayStatics.GetPlayerCharacter` 0)) :`TraceChannel` "TraceTypeQuery2" :`bTraceComplex` true :`DrawDebugType` "ForDuration" :`DrawTime` 0.1))
    (bind (_bblockinghit _binitialoverlap _time _distance _location _impactpoint _normal _impactnormal _physmat _hitactor) (`GameplayStatics.BreakHitResult` _outhit))
    (set `CableComponent.EndLocation` (- _impactpoint (`SceneComponent.K2_GetComponentLocation` (`self.Cable`))) (`self.Cable`))
    (`KismetSystemLibrary.PrintString` (`KismetSystemLibrary.GetDisplayName` _hitactor))
    (`KismetSystemLibrary.Delay` 0.05)
    (`self.Track`)))

(fn `UserConstructionScript`)