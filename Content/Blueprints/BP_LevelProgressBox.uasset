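; BP_LevelProgressBox is a checkpoint trigger that advances the level stage and saves progress when the first-person character enters it.
; Its one-time overlap registers the box in GM_SaveLoad's level state, increments Stage, and saves both inventories, player transform and stage.
; Activate then triggers the linked Gate, first reading Stage from level state if the box was not yet activated.
; ClearStage calls a stage-specific clear for stages one and two.
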(event `/Game/Blueprints/BPI_Activate.Activate`
  (if (`self.Activated`)
    (`/Game/Blueprints/BPI_Activate.Activate` (`self.Gate`))
    (else
      (set `self.Activated` true)
      (bind _asgm_save_load (cast `/Game/Blueprints/GM_SaveLoad` (`GameplayStatics.GetGameMode`)))
      (set `self.Stage` (`/Game/Blueprints/SG_LevelState.Stage` (`/Game/Blueprints/GM_SaveLoad.LevelState` _asgm_save_load)))
      (`/Game/Blueprints/BPI_Activate.Activate` (`self.Gate`)))))

(event `self.ReceiveBeginPlay`
  (bind _asgm_save_load (cast `/Game/Blueprints/GM_SaveLoad` (`GameplayStatics.GetGameMode`)))
  (set `self.GameMode` _asgm_save_load))

(event `self.Box.OnComponentBeginOverlap`
  (params (OverlappedComponent :type "PrimitiveComponent Object Reference") (OtherActor :type "Actor Object Reference") (OtherComp :type "PrimitiveComponent Object Reference") (OtherBodyIndex :type Integer) (bFromSweep :type Boolean) (SweepResult :type "HitResult Structure (by ref)"))
  (bind _asbp_first_person_character (cast `/Game/FirstPerson/Blueprints/BP_FirstPersonCharacter` OtherActor))
  (`KismetSystemLibrary.PrintText` "Yep")
  (`/Engine/EditorBlueprintResources/StandardMacros.DoOnce` (`self.Activated`)
    (:`Completed`
      (bind _asgm_save_load (cast `/Game/Blueprints/GM_SaveLoad` (`GameplayStatics.GetGameMode`)))
      (`/Game/Blueprints/SG_LevelState.AddActor` (`/Game/Blueprints/GM_SaveLoad.LevelState` _asgm_save_load) self)
      (bind _output_get (set `self.Stage` (+ (`self.Stage`) 1)))
      (`/Game/Blueprints/GM_SaveLoad.Save` (`self.GameMode`) (`/Game/Blueprints/BPC_Inventory.EnumInventory` (`/Game/FirstPerson/Blueprints/BP_FirstPersonCharacter.BPC_InvBelt` _asbp_first_person_character)) (`/Game/Blueprints/BPC_Inventory.EnumInventory` (`/Game/FirstPerson/Blueprints/BP_FirstPersonCharacter.BPC_InvBackPack` _asbp_first_person_character)) (`self.GetTransform` _asbp_first_person_character) _output_get)
      (set `self.Activated` true)
      (`/Game/Blueprints/BPI_Activate.Activate`))))

(event `Clear Stage`
  (switch `int` (`self.Stage`)
    (:`1`
      (`self.ClearStage1`))
    (:`2`
      (`self.ClearStage2`))))

(fn `UserConstructionScript`)