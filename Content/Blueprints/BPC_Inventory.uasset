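; Inventory component that stores slot contents as an array of item enums and announces changes through event dispatchers.
; GetSlot resolves a slot's enum to its full item row by linearly scanning DT_Items for a matching ItemEnum, printing any missing row names.
; SetSlot writes one entry and fires a slot-update event, while SetEnumArray replaces the whole array and fires a single grid-refresh event.
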(fn `GetItemDetails`
  (params (ItemEnum :type "/Game/Blueprints/ENUM_Items Enum" :default "NewEnumerator11"))
  (returns (ItemDetails :type "/Game/Blueprints/ST_Item Structure"))
  (bind _outrownames (`DataTableFunctionLibrary.GetDataTableRowNames` "/Game/Blueprints/DT_Items.DT_Items"))
  (for _array_element _outrownames
    (bind _returnvalue (`|GetDataTableRow` "/Game/Blueprints/DT_Items.DT_Items" _array_element)
      (:`then`
        (if (`|EnumEquality` (`.ItemEnum_21_12BD5CE744C370A084DBEA88A317A901` (break `/Game/Blueprints/ST_Item` _returnvalue)) ItemEnum)
          (return _returnvalue)))
      (:`RowNotFound`
        (`KismetSystemLibrary.PrintText` (`KismetTextLibrary.Conv_NameToText` _array_element))))))

(fn `GetSlot`
  (params (RequestedSlot :type Integer))
  (returns (ItemDetails :type "/Game/Blueprints/ST_Item Structure"))
  (return (`self.GetItemDetails` (`|GetArrayItem` (`self.EnumInventory`) RequestedSlot))))

(fn `SetEnumArray`
  (params (EnumInventory :type "Array of /Game/Blueprints/ENUM_Items Enum"))
  (set `self.EnumInventory` EnumInventory)
  (`self.OnRefreshGrid`))

(fn `SetSlot`
  (params (Item :type "/Game/Blueprints/ENUM_Items Enum" :default "NewEnumerator11") (Index :type Integer))
  (`KismetArrayLibrary.Array_Set` (`self.EnumInventory`) Index Item)
  (`self.OnSlotUpdate` Index))