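; Holdable grapple gun item that the player can pick up, fire in two modes and drop.
; Use and AltUse call Grapple and AltGrapple on BP_FirstPersonCharacter, where the grapple logic lives, and play a shot sound.
; Pickup stores the owner, disables physics and collision, snaps to player 0's HoldPoint and returns the item type.
; Drop clears the owner's HeldItem, restores physics and applies a forward force.
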(event `/Game/Blueprints/BPI_Item.Use`
  (bind _asbp_first_person_character (cast `/Game/FirstPerson/Blueprints/BP_FirstPersonCharacter` (`GameplayStatics.GetPlayerCharacter` 0)))
  (`/Game/FirstPerson/Blueprints/BP_FirstPersonCharacter.Grapple` _asbp_first_person_character)
  (`GameplayStatics.PlaySound2D` "/Game/FirstPerson/shoot.shoot" 1.0 1.0 0.0 null null))

(event `/Game/Blueprints/BPI_Item.AltUse`
  (bind _asbp_first_person_character (cast `/Game/FirstPerson/Blueprints/BP_FirstPersonCharacter` (`GameplayStatics.GetPlayerCharacter` 0)))
  (`/Game/FirstPerson/Blueprints/BP_FirstPersonCharacter.AltGrapple` _asbp_first_person_character)
  (`GameplayStatics.PlaySound2D` "/Game/FirstPerson/shoot.shoot" 1.0 1.0 0.0 null null))

(event `/Game/Blueprints/BPI_Item.Drop`
  (bind _grapplegun (`self.GrappleGun`))
  (set `/Game/Blueprints/BPC_Interact.HeldItem` null (`self.ItemOwner`))
  (`PhysicsThreadLibrary.AddForce` (struct) (* (`SceneComponent.GetForwardVector` _grapplegun) 20000.0))
  (`PrimitiveComponent.SetCollisionEnabled` _grapplegun "QueryAndPhysics")
  (`PrimitiveComponent.SetSimulatePhysics` (`self.GrappleGun`) true))

(fn `Pickup`
  (params (Owner :type "/Game/Blueprints/BPC_Interact Object Reference"))
  (returns (ItemType :type "/Game/Blueprints/ENUM_Items Enum"))
  (set `self.ItemOwner` Owner)
  (`PrimitiveComponent.SetCollisionEnabled` (`self.GrappleGun`) "NoCollision")
  (`PrimitiveComponent.SetSimulatePhysics` (`self.GrappleGun`) false)
  (`KismetSystemLibrary.PrintText` "You got me!")
  (bind _asbp_first_person_character (cast `/Game/FirstPerson/Blueprints/BP_FirstPersonCharacter` (`GameplayStatics.GetPlayerCharacter` 0)))
  (`self.K2_AttachToComponent` (`/Game/FirstPerson/Blueprints/BP_FirstPersonCharacter.HoldPoint` _asbp_first_person_character) "None" "SnapToTarget" "SnapToTarget" "KeepRelative")
  (return (`self.ItemType`)))

(fn `UserConstructionScript`)