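; BP_Key is a pickup that grants the first-person character the key identified by its Key variable.
; On begin play it creates a W_KeyLetter widget for that key and shows it on a widget component, rotated each tick to face the player camera.
; When the character overlaps its sphere, it adds the key, enables that key's button in the character's KeysOverlay, plays a pickup sound and destroys itself.
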(event `self.ReceiveBeginPlay`
  (bind _returnvalue (`|CreateWidget` "/Game/Blueprints/Widget/W_KeyLetter.W_KeyLetter_C" null (`self.Key`)))
  (bind _output_get (set `self.KeyLetterWidget` _returnvalue))
  (`WidgetComponent.SetWidget` (`self.Widget`) _output_get))

(event `self.ReceiveTick`
  (params (DeltaSeconds :type "Float (single-precision)"))
  (`SceneComponent.K2_SetWorldRotation` (`self.Widget`) (`KismetMathLibrary.FindLookAtRotation` (`SceneComponent.K2_GetComponentLocation` (`self.Widget`)) (`SceneComponent.K2_GetComponentLocation` (`PlayerCameraManager.TransformComponent` (`GameplayStatics.GetPlayerCameraManager` 0)))) false false))

(event `self.Sphere.OnComponentBeginOverlap`
  (params (OverlappedComponent :type "PrimitiveComponent Object Reference") (OtherActor :type "Actor Object Reference") (OtherComp :type "PrimitiveComponent Object Reference") (OtherBodyIndex :type Integer) (bFromSweep :type Boolean) (SweepResult :type "HitResult Structure (by ref)"))
  (bind _key (`self.Key`))
  (bind _asbp_first_person_character (cast `/Game/FirstPerson/Blueprints/BP_FirstPersonCharacter` OtherActor))
  (`/Game/FirstPerson/Blueprints/BP_FirstPersonCharacter.AddKey` _asbp_first_person_character _key)
  (`/Game/Blueprints/Widget/W_Keys.EnableButton` (`/Game/FirstPerson/Blueprints/BP_FirstPersonCharacter.KeysOverlay` _asbp_first_person_character) _key)
  (`GameplayStatics.PlaySound2D` "/Game/Audio/PickupKey_Cue.PickupKey_Cue" 1.0 1.0 0.0 null null)
  (`self.K2_DestroyActor`))

(fn `UserConstructionScript`)