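; BP_CoolThing is a pickup item that the player can hold and use up.
; Pickup prints a message, snaps the item to the first-person character's HoldPoint, disables collision on its Sphere and Cube, and tilts it.
; Use clears the owner's HeldItem reference and destroys the actor.
; An AddImpulse node is present but never runs.
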(event `/Game/Blueprints/BPI_Item.Pickup`
  (params (Owner :type "/Game/Blueprints/BPC_Interact Object Reference"))
  (`KismetSystemLibrary.PrintText` "You got me!")
  (bind _asbp_first_person_character (cast `/Game/FirstPerson/Blueprints/BP_FirstPersonCharacter` (`GameplayStatics.GetPlayerCharacter` 0)))
  (`self.K2_AttachToComponent` (`/Game/FirstPerson/Blueprints/BP_FirstPersonCharacter.HoldPoint` _asbp_first_person_character) "None" "SnapToTarget" "KeepRelative" "KeepRelative")
  (`PrimitiveComponent.SetCollisionEnabled` (`self.Sphere`) "NoCollision")
  (`PrimitiveComponent.SetCollisionEnabled` (`self.Cube`) "NoCollision")
  (`self.K2_SetActorRelativeRotation` (struct :`Yaw` 20.0)))

(event `/Game/Blueprints/BPI_Item.Use`
  (set `/Game/Blueprints/BPC_Interact.HeldItem` null (stale `/Game/Blueprints/BPI_Item.Pickup` Owner))
  (`self.K2_DestroyActor`))

(fn `UserConstructionScript`)