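; BP_Spear is a held spear item the first-person player can pick up, jab with, lunge with and drop.
; Pickup attaches it to the character's HoldPoint without collision and caches that point's relative location.
; Use plays a hit sound while the JabForward timeline slides HoldPoint forward from that location.
; AltUse launches the character along its forward vector, and Drop applies forward force and re-enables collision and physics.
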(event `/Game/Blueprints/BPI_Item.Pickup`
  (params (Owner :type "/Game/Blueprints/BPC_Interact Object Reference"))
  (`KismetSystemLibrary.PrintText` "You got me!")
  (bind _asbp_first_person_character (cast `/Game/FirstPerson/Blueprints/BP_FirstPersonCharacter` (`GameplayStatics.GetPlayerCharacter` 0)))
  (bind _holdpoint (`/Game/FirstPerson/Blueprints/BP_FirstPersonCharacter.HoldPoint` _asbp_first_person_character))
  (set `self.HoldPointRelativeLocation` (`SceneComponent.RelativeLocation` _holdpoint))
  (`self.K2_AttachToComponent` _holdpoint "None" "SnapToTarget" "KeepRelative" "KeepRelative")
  (`PrimitiveComponent.SetCollisionEnabled` (`self.Spear`) "NoCollision"))

(event `/Game/Blueprints/BPI_Item.Use`
  (bind (_holdpointrelativelocation_x _holdpointrelativelocation_y _holdpointrelativelocation_z) (`KismetMathLibrary.BreakVector` (`self.HoldPointRelativeLocation`)))
  (`GameplayStatics.PlaySound2D` "/Game/FirstPerson/spearHit.spearHit" 1.0 1.0 0.0 null null)
  (bind _asbp_first_person_character (cast `/Game/FirstPerson/Blueprints/BP_FirstPersonCharacter` (`GameplayStatics.GetPlayerCharacter` 0)))
  (bind (_direction _spearjabtrack) (`Timeline|JabForward` :!via `PlayFromStart`)
    (:`Update`
      (`SceneComponent.K2_SetRelativeLocation` (`/Game/FirstPerson/Blueprints/BP_FirstPersonCharacter.HoldPoint` _asbp_first_person_character) (`KismetMathLibrary.MakeVector` (`KismetMathLibrary.Lerp` _holdpointrelativelocation_x (+ _holdpointrelativelocation_x 100.0) _spearjabtrack) _holdpointrelativelocation_y _holdpointrelativelocation_z) false false))))

(event `/Game/Blueprints/BPI_Item.AltUse`
  (bind _asbp_first_person_character (cast `/Game/FirstPerson/Blueprints/BP_FirstPersonCharacter` (`GameplayStatics.GetPlayerCharacter` 0)))
  (`Character.LaunchCharacter` _asbp_first_person_character (* (`self.GetActorForwardVector` _asbp_first_person_character) 2000.0) false false)
  (`GameplayStatics.PlaySound2D` "/Game/FirstPerson/thrust.thrust" 1.0 1.0 0.0 null null))

(event `/Game/Blueprints/BPI_Item.Drop`
  (bind _spear (`self.Spear`))
  (`PhysicsThreadLibrary.AddForce` (struct) (* (`SceneComponent.GetForwardVector` (`self.Spear`)) 1000.0))
  (`PrimitiveComponent.SetCollisionEnabled` _spear "QueryAndPhysics")
  (`PrimitiveComponent.SetSimulatePhysics` _spear true))

(fn `UserConstructionScript`)