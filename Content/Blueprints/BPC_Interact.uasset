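; Player interaction component that handles picking up, holding, switching, using and dropping items in first person.
; A self-repeating, delayed camera sphere trace caches the looked-at BPI_Item actor, which E stores in the first open belt slot.
; Belt slot selection and updates destroy or spawn the held actor, with reselecting the active slot deselecting it.
; Key and mouse input forwards use, alt-use and drop to the held item through interface messages.
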(event `Looking`
  (bind _playercamera (`self.PlayerCamera`))
  (bind _returnvalue (`SceneComponent.K2_GetComponentLocation` _playercamera))
  ; Interaction tracing
  (bind (_outhit _returnvalue_2) (`KismetSystemLibrary.SphereTraceSingle` :`Start` _returnvalue :`End` (+ _returnvalue (* (`SceneComponent.GetForwardVector` _playercamera) 1000.0)) :`Radius` 50.0 :`TraceChannel` "TraceTypeQuery1" :`DrawTime` (`self.InteractDuration`)))
  (if _returnvalue_2
    (bind (_bblockinghit _binitialoverlap _time _distance _location _impactpoint _normal _impactnormal _physmat _hitactor) (`GameplayStatics.BreakHitResult` _outhit))
    (if (`KismetSystemLibrary.DoesImplementInterface` _hitactor "/Game/Blueprints/BPI_Item.BPI_Item_C")
      (set `self.LastTouchedActor` _hitactor)
      (else
        (set `self.LastTouchedActor` null :!label _label)))
    (else
      (goto _label)))
  (`KismetSystemLibrary.Delay` (`self.InteractDuration`))
  (`self.Looking`))

(event `self.ReceiveBeginPlay`
  ; Setup
  (bind _asbp_first_person_character (cast `/Game/FirstPerson/Blueprints/BP_FirstPersonCharacter` (`GameplayStatics.GetPlayerCharacter` 0)))
  (bind _output_get (set `self.Player` _asbp_first_person_character))
  (set `self.PlayerCamera` (`/Game/FirstPerson/Blueprints/BP_FirstPersonCharacter.FirstPersonCamera` _output_get))
  (`self.Looking`)
  (`self.Swap Active Item` 0)
  (add `/Game/Blueprints/BPC_Inventory.OnSlotUpdate` (`/Game/FirstPerson/Blueprints/BP_FirstPersonCharacter.BPC_InvBelt` (`self.Player`)) (delegate `OnSlotUpdate_Event`)))

(event `Key|E`
  (params (Key :type "Key Structure"))
  (bind _bpc_invbelt (`/Game/FirstPerson/Blueprints/BP_FirstPersonCharacter.BPC_InvBelt` (`self.Player`)))
  ; Pickup item
  (:`Pressed`
    (bind _lasttouchedactor (`self.LastTouchedActor`)
      (:`then`
        (bind (_hasemptyslot _emptyslot) (`self.GetOpenSlot` (`/Game/Blueprints/BPC_Inventory.EnumInventory` _bpc_invbelt)))
        (if _hasemptyslot
          (bind _output_get (set `self.HeldItem` _lasttouchedactor))
          (bind _itemtype (message `/Game/Blueprints/BPI_Item.Pickup` _output_get self))
          (`/Game/Blueprints/BPC_Inventory.SetSlot` _bpc_invbelt _itemtype _emptyslot)
          (`self.Swap Active Item` _emptyslot)
          (`/Game/Blueprints/Widget/W_InventoryGrid.RefreshGrid` (`/Game/Blueprints/Widget/W_Backpack.W_BeltGrid` (`/Game/FirstPerson/Blueprints/BP_FirstPersonCharacter.W_BackPack` (`self.Player`))))))
      (:`else`))))

(event `OnSlotUpdate_Event`
  (params (SlotIndex :type Integer))
  ; Setup
  (`self.Update Held item` SlotIndex))

(event `Update Held item`
  (params (NewSlot :type Integer))
  ; Belt slot updating
  (if (== (`self.ActiveSlot`) NewSlot)
    (bind (_name _itemenum _description _uiimage _actorbp) (break `/Game/Blueprints/ST_Item` (`/Game/Blueprints/BPC_Inventory.GetSlot` (`/Game/FirstPerson/Blueprints/BP_FirstPersonCharacter.BPC_InvBelt` (`self.Player`)) (stale `Swap Active Item` _output_get))))
    (if (`|EnumInequality` _itemenum "NewEnumerator11") :!label _label_2
      (bind _helditem (`self.HeldItem`)
        (:`then`
          (`Actor.K2_DestroyActor` _helditem))
        (:`else`
          _))
      (bind _returnvalue (`|SpawnActorFromClass` _actorbp (`SceneComponent.GetRelativeTransform` (`/Game/FirstPerson/Blueprints/BP_FirstPersonCharacter.HoldPoint` (`self.Player`))) "Undefined" "MultiplyWithRoot" null null))
      (bind _output_get (set `self.HeldItem` _returnvalue))
      (message `/Game/Blueprints/BPI_Item.Pickup` _output_get self)
      (else
        (bind _helditem_2 (`self.HeldItem` :!label _label_3)
          (:`then`
            (`Actor.K2_DestroyActor` _helditem_2)
            (set `self.HeldItem` null))
          (:`else`))))))

(event `TryToDrop`
  (bind _player (`self.Player`))
  ; Input
  ;; Try to drop
  (bind _helditem (`self.HeldItem`)
    (:`then`
      (message `/Game/Blueprints/BPI_Item.Drop` _helditem)
      (set `self.HeldItem` null)
      (`/Game/Blueprints/BPC_Inventory.SetSlot` (`/Game/FirstPerson/Blueprints/BP_FirstPersonCharacter.BPC_InvBelt` _player) "NewEnumerator11" (`self.ActiveSlot`))
      (`/Game/Blueprints/Widget/W_InventoryGrid.RefreshGrid` (`/Game/Blueprints/Widget/W_Backpack.W_BeltGrid` (`/Game/FirstPerson/Blueprints/BP_FirstPersonCharacter.W_BackPack` _player))))
    (:`else`)))

(event `Key|Q`
  (params (Key :type "Key Structure"))
  ; Input
  (:`Pressed`
    (`self.TryToDrop`)))

(event `Swap Active Item`
  (params (SlotIndex :type Integer))
  ; Belt slot updating
  (if (!= SlotIndex (`self.ActiveSlot`))
    (bind _output_get (set `self.ActiveSlot` SlotIndex))
    (goto _label_2)
    (else
      (set `self.ActiveSlot` -1)
      (goto _label_3))))

(event `Try To Use`
  ; Input
  ;; Try to use
  (bind _helditem (`self.HeldItem`)
    (:`then`
      (message `/Game/Blueprints/BPI_Item.Use` _helditem))
    (:`else`)))

(event `Key|LeftMouseButton`
  (params (Key :type "Key Structure"))
  ; Input
  (:`Pressed`
    (`self.Try To Use`)))

(event `TryToAltUse`
  ; Input
  ;; Try to alt use
  (bind _helditem (`self.HeldItem`)
    (:`then`
      (message `/Game/Blueprints/BPI_Item.AltUse` _helditem))
    (:`else`)))

(event `Key|RightMouseButton`
  (params (Key :type "Key Structure"))
  ; Input
  (:`Pressed`
    (`self.TryToAltUse`)))

(event `Key|One`
  (params (Key :type "Key Structure"))
  ; Belt slot updating
  ;; Swap active slot
  (:`Pressed`
    (`self.Swap Active Item` 0)))

(event `Key|Two`
  (params (Key :type "Key Structure"))
  ; Belt slot updating
  ;; Swap active slot
  (:`Pressed`
    (`self.Swap Active Item` 1)))

(event `Key|Three`
  (params (Key :type "Key Structure"))
  ; Belt slot updating
  ;; Swap active slot
  (:`Pressed`
    (`self.Swap Active Item` 2)))

(fn `GetOpenSlot`
  (params (Inventory :type "Array of /Game/Blueprints/ENUM_Items Enum"))
  (returns (HasEmptySlot :type Boolean) (EmptySlot :type Integer))
  (locals (OpenSlot :type Integer) (HasOpenSlot :type Boolean))
  (set `local.HasOpenSlot` false)
  (for (_array_element _array_index) Inventory
    (if (`|EnumEquality` _array_element "NewEnumerator11")
      (set `local.OpenSlot` _array_index)
      (set `local.HasOpenSlot` true)
      (break)))
  (return (`local.HasOpenSlot`) (`local.OpenSlot`)))