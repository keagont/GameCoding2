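; BP_FakeTree is an enemy pawn disguised as a fir tree that chases the player once seen and restarts the level on contact.
; External Decay calls build decay, causing death, sinking and destruction when full; a retriggerable delay starts regrowth when they pause.
; A looping DecayCheck maps decay to movement speed and material fade.
; Fade materials are created by a debug key or the Fadeout function, not on BeginPlay.
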(event OnSeePawn(PawnSensing)
  (params (Pawn :type Pawn%20Object%20Reference))
  (if (not (Variables|Default|GetPlayerSeen))
    (Utilities|Casting|CastToBP_FirstPersonCharacter Pawn)
    (Variables|Default|SetPlayerSeen true)
    (CallFunction|Chase)
    (Development|PrintText "Saw you" true true "(R=1.000000,G=0.289062,B=0.802681,A=1.000000)")))

(event OnComponentBeginOverlap(KillSphere)
  (params (OverlappedComponent :type Primitive%20Component%20Object%20Reference) (OtherActor :type Actor%20Object%20Reference) (OtherComp :type Primitive%20Component%20Object%20Reference) (OtherBodyIndex :type Integer) (bFromSweep :type Boolean) (SweepResult :type Hit%20Result%20Structure%20%28by%20ref%29))
  (bind _asbp_first_person_character (Utilities|Casting|CastToBP_FirstPersonCharacter OtherActor))
  (Default|RestartLevel _asbp_first_person_character))

(event Custom|Decay
  (if (not (Variables|Default|GetDead))
    (bind _output_get (Variables|Default|SetDecayAmount (+ (Variables|Default|GetDecayAmount) 0.05)))
    (Development|PrintText (Utilities|Text|FormatText "{p}% decayed" (* _output_get 1e+02)))
    (Utilities|FlowControl|Sequence
      (:then_0
        (if (>= (Variables|Default|GetDecayAmount) 1.0)
          (Variables|Default|SetDead true)
          (CallFunction|Die)))
      (:then_1
        (Utilities|FlowControl|RetriggerableDelay 1.0)
        (if (not (Variables|Default|GetDead))
          (Variables|Default|SetStartingDecay (Variables|Default|GetDecayAmount))
          (bind _regrowth (Timeline|RegrowTimeline PlayFromStart)
            (:Update
              (Variables|Default|SetDecayAmount (Math|Float|Lerp (Variables|Default|GetStartingDecay) 0.0 _regrowth)))))))))

(event Custom|Die
  (Development|PrintText "I died!")
  (Variables|/Script/Engine.FloatingPawnMovement|SetMaxSpeed (Variables|Default|GetFloatingPawnMovement) 0.0)
  (Variables|Default|SetStartingLocation (Transformation|GetActorLocation))
  (bind _sinktrack (Timeline|Timeline PlayFromStart)
    (:Update
      (Transformation|SetActorLocation (Math|Vector|MakeVector (.x (Variables|Default|GetStartingLocation)) (.y (Variables|Default|GetStartingLocation)) (Math|Float|Lerp (.z (Variables|Default|GetStartingLocation)) (- (.z (Variables|Default|GetStartingLocation)) 5e+02) _sinktrack)) false false))
    (:Finished
      (Actor|DestroyActor))))

(event Custom|Chase
  (AI|AIMoveTo self (Transformation|GetWorldLocation (Variables|/Script/Engine.Character|GetCapsuleComponent (Game|GetPlayerCharacter 0))) 0 1.0 false
    (:then
      (Utilities|FlowControl|Delay 0.5)
      (CallFunction|Chase))
    (:OnFail
      (Development|PrintText "I fail!" true true "(R=1.000000,G=0.289062,B=0.802681,A=1.000000)"))))

(event Custom|DecayCheck
  (bind _decayamount (Variables|Default|GetDecayAmount))
  (Development|PrintText "YEP" true true "(R=0.000000,G=0.660000,B=1.000000,A=1.000000)" 0.05)
  (Variables|/Script/Engine.FloatingPawnMovement|SetMaxSpeed (Variables|Default|GetFloatingPawnMovement) (Math|Float|Lerp 6e+02 0.0 _decayamount))
  (for _array_element (Variables|Default|GetDynamicMaterialInstance)
    (Rendering|Material|SetScalarParameterValue _array_element "FadeAmount" (Math|Float|Lerp -1.0 1.0 _decayamount) :!class /Script/Engine.MaterialInstanceDynamic))
  (Utilities|FlowControl|Delay 0.05)
  (CallFunction|DecayCheck))

(event EventBeginPlay
  (CallFunction|DecayCheck))

(event Input|KeyboardEvents|DebugKeyX
  (params (Key :type Key%20Structure :default "None") (ActionValue :type Input%20Action%20Value%20Structure))
  (bind _sm_fir_tree_01 (Variables|Default|GetSM_Fir_Tree_01))
  (:Pressed
    (Development|PrintString "Doing it")
    (Utilities|Array|Clear (Variables|Default|GetDynamicMaterialInstance))
    (for (_array_element _array_index) (Rendering|Material|GetMaterials _sm_fir_tree_01)
      (bind _returnvalue (Rendering|Material|CreateDynamicMaterialInstance _sm_fir_tree_01 _array_index _array_element "None" :!class /Script/Engine.PrimitiveComponent))
      (Utilities|Array|Add (Variables|Default|GetDynamicMaterialInstance) _returnvalue))))

(fn ConstructionScript)

(fn Fadeout
  (bind _sm_fir_tree_01 (Variables|Default|GetSM_Fir_Tree_01))
  (Utilities|Array|Clear (Variables|Default|GetDynamicMaterialInstance))
  (for (_array_element _array_index) (Rendering|Material|GetMaterials _sm_fir_tree_01)
    (bind _returnvalue (Rendering|Material|CreateDynamicMaterialInstance _sm_fir_tree_01 _array_index _array_element "None" :!class /Script/Engine.PrimitiveComponent))
    (Utilities|Array|Add (Variables|Default|GetDynamicMaterialInstance) _returnvalue)))