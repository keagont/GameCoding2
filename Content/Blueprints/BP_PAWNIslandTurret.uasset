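; Island turret that spins to scan for the first-person player and restarts the level when it shoots them.
; A looping Timeline drives the 360-degree scan until PawnSensing spots the player, swapping the vision cone material and starting a repeating targeting timer.
; Each tick yaws toward the player, places a cable laser by line trace and builds a score that triggers the shot.
; A retriggerable delay resumes scanning once sightings stop.
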(event `Shoot`
  (bind _cable (`self.Cable`))
  (set `self.TargetScore` 0.0)
  (bind (_outhit _returnvalue) (`KismetSystemLibrary.LineTraceSingle` (`SceneComponent.K2_GetComponentLocation` _cable) (+ (`SceneComponent.K2_GetComponentLocation` (`Character.CapsuleComponent` (`self.Player`))) (* (`SceneComponent.GetForwardVector` _cable) 100.0)) "TraceTypeQuery2"))
  (if _returnvalue
    (bind _asbp_first_person_character (cast `/Game/FirstPerson/Blueprints/BP_FirstPersonCharacter` (`.HitActor` (`GameplayStatics.BreakHitResult` _outhit))))
    (`/Game/FirstPerson/Blueprints/BP_FirstPersonCharacter.RestartLevel` _asbp_first_person_character)))

(event `RestartScan`
  (bind _startrot (`self.StartRot`))
  (set `self.TargetScore` 0.0)
  (`KismetSystemLibrary.PrintString` "Restarting")
  (`PrimitiveComponent.SetMaterial` (`self.VisualCone`) 0 "/Game/Materials/MI_TurretNoTarget.MI_TurretNoTarget")
  (`SceneComponent.SetVisibility` (`self.Cable`) false false)
  (set `self.SeenPlayer` false)
  (`self.Scan`)
  (`KismetSystemLibrary.K2_ClearAndInvalidateTimerHandle` (stale `self.PawnSensing.OnSeePawn` _returnvalue))
  (goto _label :!via `Reset`))

(event `TargetPlayer`
  (bind _cable (`self.Cable`))
  (bind _startrot (`self.StartRot`))
  (bind _returnvalue (`SceneComponent.K2_GetComponentLocation` (`Character.CapsuleComponent` (`self.Player`))))
  (bind (_returnvalue_roll _returnvalue_pitch _returnvalue_yaw) (`KismetMathLibrary.BreakRotator` (`KismetMathLibrary.FindLookAtRotation` (`self.K2_GetActorLocation`) _returnvalue)))
  (`|ExecutionSequence`
    (:`then_0`
      (`/Engine/EditorBlueprintResources/StandardMacros.DoOnce` false :!label _label
        (:`Completed`
          (bind (_direction _scantrack) (`Timeline|Timeline` :!via `Stop` :!label _label_2)
            (:`Update`
              (`self.K2_SetActorRotation` (`KismetMathLibrary.MakeRotator` 0.0 0.0 (`KismetMathLibrary.Lerp` _startrot (+ _startrot 360.0) _scantrack))))
            (:`Finished`
              (`self.Scan`))))))
    (:`then_1`
      (bind (_outhit _returnvalue_2) (`KismetSystemLibrary.LineTraceSingle` :`Start` (`SceneComponent.K2_GetComponentLocation` _cable) :`End` (+ _returnvalue (* (`SceneComponent.GetForwardVector` _cable) 100.0)) :`TraceChannel` "TraceTypeQuery2" :`bTraceComplex` true :`DrawDebugType` "ForDuration" :`DrawTime` 0.1))
      (`|ExecutionSequence`
        (:`then_0`
          (if _returnvalue_2
            (`SceneComponent.SetVisibility` (`self.Cable`) true false)
            (set `CableComponent.EndLocation` (`.ImpactPoint` (`GameplayStatics.BreakHitResult` _outhit)) (`self.Cable`))
            (else
              (`SceneComponent.SetVisibility` (`self.Cable`) false false))))
        (:`then_1`
          (`self.K2_SetActorRotation` (`KismetMathLibrary.MakeRotator` 0.0 0.0 _returnvalue_yaw))
          (bind _output_get (set `self.TargetScore` (+ (`self.TargetScore`) 1.0)))
          (if (>= _output_get 25.0)
            (`self.Shoot`)))))))

(event `self.ReceiveBeginPlay`
  (`self.Scan`)
  (`SceneComponent.SetVisibility` (`self.Cable`) false false))

(event `Scan`
  (bind (_returnvalue_roll _returnvalue_pitch _returnvalue_yaw) (`KismetMathLibrary.BreakRotator` (`self.K2_GetActorRotation`)))
  (if (not (`self.SeenPlayer`))
    (`KismetSystemLibrary.PrintText` "Scanning")
    (set `self.StartRot` _returnvalue_yaw)
    (goto _label_2 :!via `PlayFromStart`)))

(event `Attack`)

(event `self.PawnSensing.OnSeePawn`
  (params (Pawn :type "Pawn Object Reference"))
  (bind _asbp_first_person_character (cast `/Game/FirstPerson/Blueprints/BP_FirstPersonCharacter` Pawn)
    (:`then`
      (set `self.Player` _asbp_first_person_character)
      (`KismetSystemLibrary.PrintText` "I see You")
      (`|ExecutionSequence`
        (:`then_0`
          (`/Engine/EditorBlueprintResources/StandardMacros.DoOnce` false :!label _label_3
            (:`Completed`
              (set `self.SeenPlayer` true)
              (`PrimitiveComponent.SetMaterial` (`self.VisualCone`) 0 "/Game/Materials/MI_TurretFoundTarget.MI_TurretFoundTarget")
              (`self.TargetPlayer`)
              (bind _returnvalue (`KismetSystemLibrary.K2_SetTimerDelegate` (delegate `TargetPlayer`) 0.1 true))
              (`SceneComponent.SetVisibility` (`self.Cable`) true false))))
        (:`then_1`
          (`KismetSystemLibrary.RetriggerableDelay` 1.5)
          (`self.RestartScan`)
          (goto _label_3 :!via `Reset`))))
    (:`CastFailed`
      (`KismetSystemLibrary.PrintText` "IM DUMB!"))))

(fn `UserConstructionScript`)