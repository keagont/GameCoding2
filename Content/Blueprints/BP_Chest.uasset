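; Chest actor that exposes its BPCInventory to the player's backpack UI when the first-person character walks into its sphere.
; Overlap raises the lid, prints the first item, hands the inventory to WBackPack and fills it after a zero delay; leaving reverses lid and display.
; BeginPlay also creates a chest widget, unused in these graphs.
; Use forwards to the player's held BP_CoolThing, while Pickup just returns a fixed enum value.
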(event `/Game/Blueprints/BPI_Item.Use`
  (bind _asbp_first_person_character (cast `/Game/FirstPerson/Blueprints/BP_FirstPersonCharacter` (`GameplayStatics.GetPlayerCharacter` 0)))
  (bind _asbp_cool_thing (cast `/Game/Blueprints/BP_CoolThing` (`/Game/Blueprints/BPC_Interact.HeldItem` (`/Game/FirstPerson/Blueprints/BP_FirstPersonCharacter.BPC_Interact` _asbp_first_person_character))))
  (`/Game/Blueprints/BPI_Item.Use` _asbp_cool_thing))

(event `self.ReceiveBeginPlay`
  (bind _returnvalue (`|CreateWidget` "/Game/Blueprints/Widget/W_ChestInventory.W_ChestInventory_C" null (`self.BPC_Inventory`)))
  (set `self.InventoryWidget` _returnvalue))

(event `self.Sphere.OnComponentBeginOverlap`
  (params (OverlappedComponent :type "PrimitiveComponent Object Reference") (OtherActor :type "Actor Object Reference") (OtherComp :type "PrimitiveComponent Object Reference") (OtherBodyIndex :type Integer) (bFromSweep :type Boolean) (SweepResult :type "HitResult Structure (by ref)"))
  (bind _chesttop (`self.ChestTop`))
  (bind (_returnvalue_x _returnvalue_y _returnvalue_z) (`KismetMathLibrary.BreakVector` (`SceneComponent.K2_GetComponentLocation` _chesttop)))
  (bind (_name _itemenum _description) (break `/Game/Blueprints/ST_Item` (`|GetArrayItem` (`/Game/Blueprints/BPC_Inventory.Inventory` (`self.BPC_Inventory`)))))
  (bind _asbp_first_person_character (cast `/Game/FirstPerson/Blueprints/BP_FirstPersonCharacter` OtherActor))
  (`KismetSystemLibrary.PrintText` (`|FormatText` "The first item is {name}: {desc}" _name _description))
  (`SceneComponent.K2_SetWorldLocation` _chesttop (`KismetMathLibrary.MakeVector` _returnvalue_x _returnvalue_y (+ _returnvalue_z 20.0)) false false)
  (bind _w_backpack (`/Game/FirstPerson/Blueprints/BP_FirstPersonCharacter.W_BackPack` _asbp_first_person_character))
  (`/Game/Blueprints/Widget/W_Backpack.SetChestInv` _w_backpack (`self.BPC_Inventory`))
  (`KismetSystemLibrary.Delay` 0.0)
  (`/Game/Blueprints/Widget/W_InventoryPanel.AddAllItems` (`/Game/Blueprints/Widget/W_Backpack.W_ChestInv` _w_backpack))
  (`/Game/Blueprints/Widget/W_Backpack.ShowChest` _w_backpack))

(event `self.Sphere.OnComponentEndOverlap`
  (params (OverlappedComponent :type "PrimitiveComponent Object Reference") (OtherActor :type "Actor Object Reference") (OtherComp :type "PrimitiveComponent Object Reference") (OtherBodyIndex :type Integer))
  (bind _chesttop (`self.ChestTop`))
  (bind (_returnvalue_x _returnvalue_y _returnvalue_z) (`KismetMathLibrary.BreakVector` (`SceneComponent.K2_GetComponentLocation` _chesttop)))
  (bind _asbp_first_person_character (cast `/Game/FirstPerson/Blueprints/BP_FirstPersonCharacter` OtherActor))
  (`/Game/Blueprints/Widget/W_Backpack.HideChest` (`/Game/FirstPerson/Blueprints/BP_FirstPersonCharacter.W_BackPack` _asbp_first_person_character))
  (`SceneComponent.K2_SetWorldLocation` _chesttop (`KismetMathLibrary.MakeVector` _returnvalue_x _returnvalue_y (+ _returnvalue_z -20.0)) false false))

(fn `Pickup`
  (params (Owner :type "/Game/Blueprints/BPC_Interact Object Reference"))
  (returns (ItemType :type "/Game/Blueprints/ENUM_Items Enum"))
  (return "NewEnumerator11"))

(fn `UserConstructionScript`)