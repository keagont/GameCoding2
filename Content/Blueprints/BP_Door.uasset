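; BP_Door is a locked door that opens when the first-person character enters its sphere trigger carrying the needed keys.
; On BeginPlay it creates a W_Name widget, sets it up with the required keys and shows it on its widget component.
; On overlap the character checks the keys: failure plays a bad-keys sound, while success triggers the widget's unlock, waits in proportion to key count, snaps the cube's rotation, plays a sound and unlocks.
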(event `self.ReceiveBeginPlay`
  (bind _returnvalue (`|CreateWidget` "/Game/Blueprints/Widget/W_Name.W_Name_C"))
  (bind _output_get (set `self.WName` _returnvalue))
  (`/Game/Blueprints/Widget/W_Name.Setup Name` _output_get (`self.Needed Keys`))
  (`WidgetComponent.SetWidget` (`self.Widget`) _output_get))

(event `self.Sphere.OnComponentBeginOverlap`
  (params (OverlappedComponent :type "PrimitiveComponent Object Reference") (OtherActor :type "Actor Object Reference") (OtherComp :type "PrimitiveComponent Object Reference") (OtherBodyIndex :type Integer) (bFromSweep :type Boolean) (SweepResult :type "HitResult Structure (by ref)"))
  (if (`self.Locked`)
    (bind _asbp_first_person_character (cast `/Game/FirstPerson/Blueprints/BP_FirstPersonCharacter` OtherActor))
    (bind _haskeys (`/Game/FirstPerson/Blueprints/BP_FirstPersonCharacter.CheckDoor` _asbp_first_person_character (`self.Needed Keys`)))
    (if _haskeys
      (`/Game/Blueprints/Widget/W_Name.UnlockDoor` (`self.WName`))
      (`KismetSystemLibrary.Delay` (+ (* (`KismetArrayLibrary.Array_Length` (`self.Needed Keys`)) 0.4) 1.0))
      (`SceneComponent.K2_SetWorldRotation` (`self.Cube`) (struct :`Yaw` -90.0) false false)
      (`GameplayStatics.PlaySound2D` "/Game/Audio/DoorOpen_Cue.DoorOpen_Cue" 1.0 1.0 0.0 null null)
      (set `self.Locked` false)
      (else
        (`GameplayStatics.PlaySound2D` "/Game/Audio/BadKeys_Cue.BadKeys_Cue" 1.0 1.0 0.0 null null)))))

(fn `UserConstructionScript`)