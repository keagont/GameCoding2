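; BP_RandomSetter holds a random stream that is seeded from the seed stored in the GI_SeedTest game instance.
; On BeginPlay it casts the game instance and applies that seed to its RandomNumber stream.
; The NewLevelStreamFromSeed event reseeds the stream with a number drawn from the stream itself, chaining deterministic seeds from the original, and prints a debug message.
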(event `self.ReceiveBeginPlay`
  (bind _asgi_seed_test (cast `/Game/Blueprints/GI_SeedTest` (`GameplayStatics.GetGameInstance`)))
  (`KismetMathLibrary.SetRandomStreamSeed` (`self.RandomNumber`) (`/Game/Blueprints/GI_SeedTest.Seed` _asgi_seed_test)))

(event `NewLevelStreamFromSeed`
  (`KismetMathLibrary.SetRandomStreamSeed` (`self.RandomNumber`) (`KismetMathLibrary.RandomIntegerInRangeFromStream` (`self.RandomNumber`) 100000 9999999))
  (`KismetSystemLibrary.PrintString` "Doing something new" true true (struct :`R` 1.0 :`B` 0.394135 :`A` 1.0) 20.0))

(fn `UserConstructionScript`)