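; GI_SeedTest holds a seed value and advances it through a repeatable pseudo-random sequence.
; SetSeed stores the given seed, or picks a random seven-digit one when given zero.
; AdvanceSeed reseeds a random stream with the current seed and draws the next seven-digit seed from it, so each starting seed always yields the same chain.
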(event `SetSeed`
  (params (Seed :type Integer))
  (if (== Seed 0)
    (set `self.Seed` (`KismetMathLibrary.RandomIntegerInRange` 1000000 9999999))
    (else
      (set `self.Seed` Seed))))

(event `AdvanceSeed`
  (`KismetMathLibrary.SetRandomStreamSeed` (`self.SeedStream`) (`self.Seed`))
  (set `self.Seed` (`KismetMathLibrary.RandomIntegerInRangeFromStream` (`self.SeedStream`) 1000000 9999999)))