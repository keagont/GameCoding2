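; BP_Turret is a placeable turret that follows the player's TurretPlacement component while being placed, then scans for pawns.
; Once placed, it switches to metal material and sweeps 45 degrees either side of its yaw via a looping timeline.
; Seeing any pawn stops the sweep and yaws it toward the player; a retriggerable delay behind a DoOnce later resumes scanning.
; Shooting is only a flag with no firing logic, and Cancel destroys the actor.
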(event `self.ReceiveBeginPlay`
  (bind _asbp_first_person_character (cast `/Game/FirstPerson/Blueprints/BP_FirstPersonCharacter` (`GameplayStatics.GetPlayerCharacter` 0)))
  (set `self.Player` _asbp_first_person_character))

(event `self.ReceiveTick`
  (params (DeltaSeconds :type "Float (single-precision)"))
  (bind (_returnvalue_roll _returnvalue_pitch _returnvalue_yaw) (`KismetMathLibrary.BreakRotator` (`SceneComponent.K2_GetComponentRotation` (`self.CapsuleComponent`))))
  (bind _turretplacement (`/Game/FirstPerson/Blueprints/BP_FirstPersonCharacter.TurretPlacement` (`self.Player`)))
  (if (`self.Placing`)
    (`SceneComponent.K2_SetWorldLocation` (`self.CapsuleComponent`) (`SceneComponent.K2_GetComponentLocation` _turretplacement) false false)
    (`self.K2_SetActorRotation` (`SceneComponent.K2_GetComponentRotation` _turretplacement))
    (elif (`self.Placed`)
      (if (`self.Shooting`)
        _)
      (else
        (`PrimitiveComponent.SetMaterial` (`self.Cylinder`) 0 "/Game/Materials/M_Metal.M_Metal")
        (`PrimitiveComponent.SetMaterial` (`self.StaticMesh`) 0 "/Game/Materials/M_Metal.M_Metal")
        (set `self.Placed` true)
        (set `self.LeftTurn` (- _returnvalue_yaw 45.0))
        (set `self.RightTurn` (+ _returnvalue_yaw 45.0))
        (set `self.Scanning` true)
        (`self.Scan`)))))

(event `Scan`
  (if (`self.Scanning`)
    (bind (_direction _scantrack) (`Timeline|ScanTimeline` :!via `PlayFromStart` :!label _label)
      (:`Update`
        (`self.K2_SetActorRotation` (`KismetMathLibrary.MakeRotator` 0.0 0.0 (`KismetMathLibrary.Lerp` (`self.LeftTurn`) (`self.RightTurn`) _scantrack))))
      (:`Finished`
        (`self.Scan`)))
    (else
      (goto _label :!via `Stop`))))

(event `StopScanning`
  (goto _label :!via `Stop`))

(event `self.PawnSensing.OnSeePawn`
  (params (Pawn :type "Pawn Object Reference"))
  (bind (_returnvalue_roll _returnvalue_pitch _returnvalue_yaw) (`KismetMathLibrary.BreakRotator` (`KismetMathLibrary.FindLookAtRotation` (`SceneComponent.K2_GetComponentLocation` (`self.CapsuleComponent`)) (`SceneComponent.K2_GetComponentLocation` (`Character.CapsuleComponent` (`self.Player`))))))
  (cast `/Game/FirstPerson/Blueprints/BP_FirstPersonCharacter` Pawn
    (:`then`
      _)
    (:`CastFailed`
      _))
  (`KismetSystemLibrary.PrintString` "I See You")
  (set `self.Scanning` false)
  (`self.StopScanning`)
  (set `self.Shooting` true)
  (`SceneComponent.K2_SetWorldRotation` (`self.CapsuleComponent`) (`KismetMathLibrary.MakeRotator` 0.0 0.0 _returnvalue_yaw) false false)
  (`/Engine/EditorBlueprintResources/StandardMacros.DoOnce` false :!label _label_2
    (:`Completed`
      (`KismetSystemLibrary.RetriggerableDelay` 5.0)
      (`KismetSystemLibrary.PrintString` "Scanning")
      (set `self.Shooting` false)
      (set `self.Scanning` true)
      (`self.Scan`)
      (goto _label_2 :!via `Reset`))))

(event `Cancel`
  (`self.K2_DestroyActor`))

(fn `UserConstructionScript`)