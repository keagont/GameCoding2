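; BP_Checkpoint is a checkpoint actor that saves the player's inventory when the first-person character overlaps it.
; On BeginPlay it casts the game mode to GM_SaveLoad and caches the reference.
; On overlap it passes the EnumInventory values from the character's belt and backpack components to that game mode's Save function.
; The overlap has no one-shot guard, so each entry saves again.
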(event `self.ReceiveBeginPlay`
  (bind _asgm_save_load (cast `/Game/Blueprints/GM_SaveLoad` (`GameplayStatics.GetGameMode`)))
  (set `self.GameMode` _asgm_save_load))

(event `self.ReceiveActorBeginOverlap`
  (params (OtherActor :type "Actor Object Reference"))
  (bind _asbp_first_person_character (cast `/Game/FirstPerson/Blueprints/BP_FirstPersonCharacter` OtherActor))
  (`/Game/Blueprints/GM_SaveLoad.Save` :`self` (`self.GameMode`) :`Belt` (`/Game/Blueprints/BPC_Inventory.EnumInventory` (`/Game/FirstPerson/Blueprints/BP_FirstPersonCharacter.BPC_InvBelt` _asbp_first_person_character)) :`Inv` (`/Game/Blueprints/BPC_Inventory.EnumInventory` (`/Game/FirstPerson/Blueprints/BP_FirstPersonCharacter.BPC_InvBackPack` _asbp_first_person_character))))

(fn `UserConstructionScript`)