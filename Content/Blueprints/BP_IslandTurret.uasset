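; BP_IslandTurret is a turret that scans by yawing through a full turn on a repeating timeline.
; Disconnected logic would lock onto a seen first-person character, re-aim on a looping timer and resume scanning after a retriggerable delay.
; As wired, pawn sensing only prints a debug message, so targeting never starts.
; Attack is empty, and the target-state material swaps are also unconnected.
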(event `RestartScan`
  (bind _startrot (`self.StartRot`))
  (set `self.SeenPlayer` false)
  (`self.Scan`)
  (goto _label :!via `Reset`))

(event `TargetPlayer`
  (bind _startrot (`self.StartRot`))
  (bind (_returnvalue_roll _returnvalue_pitch _returnvalue_yaw) (`KismetMathLibrary.BreakRotator` (`KismetMathLibrary.FindLookAtRotation` (`self.K2_GetActorLocation`) (`SceneComponent.K2_GetComponentLocation` (`Character.CapsuleComponent` (`self.Player`))))))
  (`|ExecutionSequence`
    (:`then_0`
      (`/Engine/EditorBlueprintResources/StandardMacros.DoOnce` false :!label _label
        (:`Completed`
          (bind (_direction _scantrack) (`Timeline|Timeline` :!via `Stop` :!label _label_2)
            (:`Update`
              (`self.K2_SetActorRotation` (`KismetMathLibrary.MakeRotator` 0.0 0.0 (`KismetMathLibrary.Lerp` _startrot (+ _startrot 360.0) _scantrack))))
            (:`Finished`
              (`self.Scan`))))))
    (:`then_1`
      (`self.K2_SetActorRotation` (`KismetMathLibrary.MakeRotator` 0.0 0.0 _returnvalue_yaw)))))

(event `self.ReceiveBeginPlay`
  (`self.Scan`))

(event `Scan`
  (bind (_returnvalue_roll _returnvalue_pitch _returnvalue_yaw) (`KismetMathLibrary.BreakRotator` (`self.K2_GetActorRotation`)))
  (if (not (`self.SeenPlayer`))
    (set `self.StartRot` _returnvalue_yaw)
    (goto _label_2 :!via `PlayFromStart`)))

(event `Attack`)

(event `self.PawnSensing.OnSeePawn`
  (params (Pawn :type "Pawn Object Reference"))
  (`KismetSystemLibrary.PrintText` "SENSING SOMETHING"))

(fn `UserConstructionScript`)