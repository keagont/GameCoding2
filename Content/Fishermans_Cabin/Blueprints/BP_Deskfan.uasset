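; BP_Deskfan is a desk fan prop with a spinning blade and configurable button positions.
; The construction script offsets four button meshes vertically by per-button height variables and pitches the blade mesh to a set starting angle.
; On BeginPlay, a RotatingMovement component targets only the blade mesh and spins it at RotateSpeed, with no Tick logic.
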(event `self.ReceiveBeginPlay`
  (bind _rotatingmovement (`self.RotatingMovement`))
  (`MovementComponent.SetUpdatedComponent` _rotatingmovement (`self.SM_Deskfan_02`))
  (set `RotatingMovementComponent.RotationRate` (`self.RotateSpeed`) _rotatingmovement))

(event `self.ReceiveTick`
  (params (DeltaSeconds :type "Float (single-precision)")))

(fn `UserConstructionScript`
  (`SceneComponent.K2_AddLocalOffset` (`self.SM_Deskfan_03`) (`KismetMathLibrary.MakeVector` 0.0 0.0 (`self.Button 1 Height`)) false false)
  (`SceneComponent.K2_AddLocalOffset` (`self.SM_Deskfan_04`) (`KismetMathLibrary.MakeVector` 0.0 0.0 (`self.Button 2 Height`)) false false)
  (`SceneComponent.K2_AddLocalOffset` (`self.SM_Deskfan_05`) (`KismetMathLibrary.MakeVector` 0.0 0.0 (`self.Button 3 Height`)) false false)
  (`SceneComponent.K2_AddLocalOffset` (`self.SM_Deskfan_06`) (`KismetMathLibrary.MakeVector` 0.0 0.0 (`self.Button 4 Height`)) false false)
  (`SceneComponent.K2_AddLocalRotation` (`self.SM_Deskfan_02`) (`KismetMathLibrary.MakeRotator` 0.0 (`self.Blade Rotation Angle`)) false false))