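; BP_Metal_Tins is a configurable metal tin prop in the Fishermans_Cabin content, built from separate base and lid static mesh components.
; The construction script uses the MetalTin selection to pick matching meshes from TinBase and TinLid, and hides the lid when HideLid is set.
; The event graph holds only disabled placeholder events, so the prop has no runtime logic.
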(fn `UserConstructionScript`
  (bind _metal_tin (`self.Metal Tin`))
  (`StaticMeshComponent.SetStaticMesh` (`self.SM_Tin_01_Base`) (`|GetArrayItem` (`self.TinBase`) _metal_tin))
  (`StaticMeshComponent.SetStaticMesh` (`self.SM_Tin_01_Lid`) (`|GetArrayItem` (`self.TinLid`) _metal_tin))
  (if (`self.Hide Lid`)
    (`SceneComponent.SetVisibility` (`self.SM_Tin_01_Lid`) false false)))