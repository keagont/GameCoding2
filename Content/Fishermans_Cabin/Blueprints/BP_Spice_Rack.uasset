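; BP_Spice_Rack is a configurable spice container prop for the Fisherman's Cabin set, built entirely in the Construction Script.
; ContainerType picks matching meshes for the container, lid, plastic insert and its flap from parallel arrays, while ContainerSpiceType picks the spice mesh.
; Exposed values offset the spice fill height, rotate the plastic insert, open its flap and toggle lid visibility along with its children.
; It has no runtime logic.
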(fn `UserConstructionScript`
  (bind _container_type (`self.Container Type`))
  (`StaticMeshComponent.SetStaticMesh` (`self.Spice_Container`) (`|GetArrayItem` (`self.Spice_Container_Array`) _container_type))
  (`StaticMeshComponent.SetStaticMesh` (`self.Spice_Container_Lid`) (`|GetArrayItem` (`self.Spice_Container_Lid_Array`) _container_type))
  (`StaticMeshComponent.SetStaticMesh` (`self.Spice_Container_Lid_PlasticPart`) (`|GetArrayItem` (`self.Spice_Container_Lid_PlasticPart_Array`) _container_type))
  (`StaticMeshComponent.SetStaticMesh` (`self.Spice_Container_Lid_PlasticPart_Lid`) (`|GetArrayItem` (`self.Spice_Container_Lid_PlasticPart_Lid_Array`) _container_type))
  (`StaticMeshComponent.SetStaticMesh` (`self.Spice`) (`|GetArrayItem` (`self.Spice_Array`) (`self.Container Spice Type`)))
  (`SceneComponent.K2_AddRelativeLocation` (`self.Spice`) (`KismetMathLibrary.MakeVector` 0.0 0.0 (`self.Spice Height Level`)) false false)
  (`SceneComponent.K2_AddLocalRotation` (`self.Spice_Container_Lid_PlasticPart`) (`KismetMathLibrary.MakeRotator` 0.0 0.0 (`self.Lid Rotation`)) false false)
  (`SceneComponent.K2_AddLocalRotation` (`self.Spice_Container_Lid_PlasticPart_Lid`) (`KismetMathLibrary.MakeRotator` (`self.Lid Open Angle`)) false false)
  (`SceneComponent.SetVisibility` (`self.Spice_Container_Lid`) (`self.Lid Visibility`) true))