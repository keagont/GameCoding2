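; BP_Glass_Jars is a configurable glass jar prop in the Fishermans_Cabin content, with a glass body, lid and optional noodle filling.
; The construction script uses GlassJarVersion to pick meshes for both glass components, with the Jars array feeding GlassLid and Lids feeding Glass.
; The same version selects the small, mid or large noodle array, NoodleVariation picks its mesh, and NoodlesVisible toggles visibility.
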(fn `UserConstructionScript`
  (bind _glass_jar_version (`self.Glass Jar Version`))
  (`StaticMeshComponent.SetStaticMesh` (`self.GlassLid`) (`|GetArrayItem` (`self.Jars`) _glass_jar_version))
  (`StaticMeshComponent.SetStaticMesh` (`self.Glass`) (`|GetArrayItem` (`self.Lids`) _glass_jar_version))
  (`StaticMeshComponent.SetStaticMesh` (`self.Noodles`) (`|GetArrayItem` (select `int` _glass_jar_version :`0` (`self.Noodles_Small`) :`1` (`self.Noodles_Mid`) :`2` (`self.Noodles_Large`)) (`self.Noodle Variation`)))
  (`SceneComponent.SetVisibility` (`self.Noodles`) (`self.Noodles Visible?`) false))