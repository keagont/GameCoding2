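; BP_Satelite_Dish is a configurable satellite dish prop whose pose is set in the Construction Script.
; An Orientation switch picks one of three layouts by hiding two of the three variant meshes (03, 04, 05), repositioning mesh 01 and pitching mesh 02.
; Each layout takes its pitch from its own variable.
; The event graph holds only disabled stub events, so the actor has no runtime logic.
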(fn `UserConstructionScript`
  (bind _sm_satelite_dish_02 (`self.SM_Satelite_Dish_02`))
  (switch `int` (`self.Orientation`)
    (:`Default`
      (`SceneComponent.SetVisibility` (`self.SM_Satelite_Dish_05`) false false)
      (`SceneComponent.SetVisibility` (`self.SM_Satelite_Dish_04`) false false)
      (`SceneComponent.K2_SetRelativeLocation` (`self.SM_Satelite_Dish_01`) (-16.597189 0.0 10.558341) false false)
      (`SceneComponent.K2_SetRelativeRotation` _sm_satelite_dish_02 (`KismetMathLibrary.MakeRotator` 0.0 (`self.Y (Pitch)`)) false false))
    (:`0`
      (`SceneComponent.SetVisibility` (`self.SM_Satelite_Dish_03`) false false)
      (`SceneComponent.SetVisibility` (`self.SM_Satelite_Dish_04`) false false)
      (`SceneComponent.K2_SetRelativeLocation` (`self.SM_Satelite_Dish_01`) (12.233656 0.0 -7.260827) false false)
      (`SceneComponent.K2_SetRelativeRotation` _sm_satelite_dish_02 (`KismetMathLibrary.MakeRotator` 0.0 (`self.Y 0`)) false false))
    (:`1`
      (`SceneComponent.SetVisibility` (`self.SM_Satelite_Dish_05`) false false)
      (`SceneComponent.SetVisibility` (`self.SM_Satelite_Dish_03`) false false)
      (`SceneComponent.K2_SetRelativeLocation` (`self.SM_Satelite_Dish_01`) (1.516041 0.0 1.823627) false false)
      (`SceneComponent.K2_SetRelativeRotation` _sm_satelite_dish_02 (`KismetMathLibrary.MakeRotator` 0.0 (`self.Y 1`)) false false))))