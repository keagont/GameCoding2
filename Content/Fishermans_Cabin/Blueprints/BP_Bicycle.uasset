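; Configurable bicycle prop assembled from separate mesh components, with adjustable pose, grips, flat tires, color and headlight glow.
; The construction script offsets and rotates parts, swaps tire meshes and sets dynamic material parameters.
; It then calls Randomize, which optionally derives pose, grips and color from Seed, so new values land after the current pass applies them.
; RandomSeed rerolls Seed; each draw makes a fresh stream from it, so values correlate.
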(event `Randomize Seed`
  (set `self.Seed` (`KismetMathLibrary.RandomIntegerInRange` 0 999999)))

(event `Randomize`
  (bind _returnvalue (`KismetMathLibrary.MakeRandomStream` (`self.Seed`)))
  (if (`self.Randomize Values?`)
    (set `self.Seat Rotation` (`KismetMathLibrary.RandomFloatInRangeFromStream` _returnvalue -15.0 15.0))
    (set `self.Seat Height` (`KismetMathLibrary.RandomFloatInRangeFromStream` _returnvalue -4.0 2.5))
    (set `self.Steering Angle` (`KismetMathLibrary.RandomFloatInRangeFromStream` _returnvalue -25.0 25.0))
    (set `self.Show Rubber Handle Grip  [Right]` (`KismetMathLibrary.RandomBoolFromStream` _returnvalue))
    (set `self.Show Rubber Handle Grip  [Left]` (`KismetMathLibrary.RandomBoolFromStream` _returnvalue))
    (set `self.Pedal Rotation` (`KismetMathLibrary.RandomFloatInRangeFromStream` _returnvalue 0.0 360.0))
    (if (`self.Randomize Color?`)
      (set `self.Bicycle Color` (`KismetMathLibrary.Conv_VectorToLinearColor` (`KismetMathLibrary.MakeVector` (`KismetMathLibrary.RandomFloatInRangeFromStream` _returnvalue 0.0 0.5) (`KismetMathLibrary.RandomFloatInRangeFromStream` _returnvalue 0.0 0.5) (`KismetMathLibrary.RandomFloatInRangeFromStream` _returnvalue 0.0 0.5)))))))

(fn `RandomSeed`
  (`self.Randomize Seed`))

(fn `UserConstructionScript`
  (bind _bicycle_010 (`self.Bicycle_010`))
  (bind _bicycle_color (`self.Bicycle Color`))
  (bind _returnvalue (`KismetMathLibrary.MakeRotator` (`self.Pedal Rotation`)))
  (bind _returnvalue_2 (* _returnvalue -1.0))
  ;[1 1 1] Seat
  (`SceneComponent.K2_AddLocalOffset` _bicycle_010 (`KismetMathLibrary.MakeVector` 0.0 0.0 (`self.Seat Height`)) false false)
  (`SceneComponent.K2_AddLocalRotation` _bicycle_010 (`KismetMathLibrary.MakeRotator` 0.0 0.0 (`self.Seat Rotation`)) false false)
  ;[1 1 1] Pedal
  (`SceneComponent.K2_AddLocalRotation` (`self.Pedal`) _returnvalue false false)
  (`SceneComponent.K2_AddLocalRotation` (`self.Bicycle_10`) _returnvalue_2 false false)
  (`SceneComponent.K2_AddLocalRotation` (`self.Bicycle_011`) _returnvalue_2 false false)
  ;[1 1 1] Steering
  (`SceneComponent.K2_AddLocalRotation` (`self.Bicycle_02`) (`KismetMathLibrary.MakeRotator` 0.0 0.0 (`self.Steering Angle`)) false false)
  (`SceneComponent.SetVisibility` (`self.Bicycle_04`) (`self.Show Rubber Handle Grip  [Right]`) false)
  (`SceneComponent.SetVisibility` (`self.Bicycle_03`) (`self.Show Rubber Handle Grip  [Left]`) false)
  ;[1 1 1] Wheels
  (`SceneComponent.K2_AddLocalRotation` (`self.Bicycle_07`) (`KismetMathLibrary.MakeRotator` (`self.Front Wheel Spokes Rotation`)) false false)
  (`SceneComponent.K2_AddLocalRotation` (`self.Bicycle_08`) (`KismetMathLibrary.MakeRotator` (`self.Back Wheel Spokes Rotation`)) false false)
  (`SceneComponent.K2_AddLocalRotation` (`self.Bicycle_06`) (`KismetMathLibrary.MakeRotator` (`self.Front Wheel Tire Rotation`)) false false)
  (`SceneComponent.K2_AddLocalRotation` (`self.Bicycle_09`) (`KismetMathLibrary.MakeRotator` (`self.Back Wheel Tire Rotation`)) false false)
  (if (`self.Enable Flat Front Tire?`)
    (`StaticMeshComponent.SetStaticMesh` (`self.Bicycle_06`) "/Game/Fishermans_Cabin/Meshes/Bicycle/SM_Bicycle_05.SM_Bicycle_05"))
  (if (`self.Enable Flat Back Tire?`)
    (`StaticMeshComponent.SetStaticMesh` (`self.Bicycle_09`) "/Game/Fishermans_Cabin/Meshes/Bicycle/SM_Bicycle_05.SM_Bicycle_05"))
  ;[1 1 1] Color
  (bind _returnvalue_3 (`PrimitiveComponent.CreateDynamicMaterialInstance` (`self.Bicycle_01`) 0 null "None"))
  (`MaterialInstanceDynamic.SetVectorParameterValue` _returnvalue_3 "Mask Color" _bicycle_color)
  (bind _returnvalue_4 (`PrimitiveComponent.CreateDynamicMaterialInstance` (`self.Bicycle_02`) 0 null "None"))
  (`MaterialInstanceDynamic.SetVectorParameterValue` _returnvalue_4 "Mask Color" _bicycle_color)
  (`MaterialInstanceDynamic.SetScalarParameterValue` _returnvalue_4 "Emissive Multiply" (`self.Headlight Intensity`))
  (`self.Randomize`))