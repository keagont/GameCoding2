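; Kitchen counter prop for the Fisherman's Cabin set, with posable doors, drawers, hanging cabinet doors, a faucet and hot and cold water wheels.
; The Construction Script applies per-part angle and offset variables as relative or local rotations and translations to mesh components, negating some to mirror opening direction.
; Posing happens only at construction, as the event graph has no active runtime logic.
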(fn `UserConstructionScript`
  (`SceneComponent.K2_AddRelativeRotation` (`self.SM_Kitchen_Counter_09`) (`KismetMathLibrary.MakeRotator` 0.0 0.0 (`self.Left Door Open Angle`)) false false)
  (`SceneComponent.K2_AddRelativeRotation` (`self.SM_Kitchen_Counter_08`) (`KismetMathLibrary.MakeRotator` 0.0 0.0 (* (`self.Right Door Open Angle`) -1.0)) false false)
  (`SceneComponent.K2_AddRelativeLocation` (`self.SM_Kitchen_Counter_07`) (`KismetMathLibrary.MakeVector` (* (`self.Top Drawer Offset`) -1.0)) false false)
  (`SceneComponent.K2_AddRelativeLocation` (`self.SM_Kitchen_Counter_06`) (`KismetMathLibrary.MakeVector` (* (`self.Middle Drawer Offset`) -1.0)) false false)
  (`SceneComponent.K2_AddRelativeLocation` (`self.SM_Kitchen_Counter_05`) (`KismetMathLibrary.MakeVector` (* (`self.Bottom Drawer Offset`) -1.0)) false false)
  (`SceneComponent.K2_AddRelativeRotation` (`self.SM_Kitchen_Counter_04`) (`KismetMathLibrary.MakeRotator` 0.0 0.0 (`self.Left Door Open Angle [R]`)) false false)
  (`SceneComponent.K2_AddRelativeRotation` (`self.SM_Kitchen_Counter_03`) (`KismetMathLibrary.MakeRotator` 0.0 0.0 (* (`self.Right Door Open Angle [R]`) -1.0)) false false)
  (`SceneComponent.K2_AddRelativeLocation` (`self.SM_Kitchen_Counter_02`) (`KismetMathLibrary.MakeVector` 0.0 (* (`self.Top Drawer Offset [R]`) -1.0)) false false)
  (`SceneComponent.K2_AddRelativeRotation` (`self.Kitchen_Addons_16`) (`KismetMathLibrary.MakeRotator` 0.0 0.0 (`self.Faucet Rotation`)) false false)
  (`SceneComponent.K2_AddLocalRotation` (`self.Kitchen_Addons_15`) (`KismetMathLibrary.MakeRotator` 0.0 0.0 (`self.Cool Water Faucet Wheel Rotation`)) false false)
  (`SceneComponent.K2_AddLocalRotation` (`self.Kitchen_Addons_18`) (`KismetMathLibrary.MakeRotator` 0.0 0.0 (`self.Hot Water Faucet Wheel Rotation`)) false false)
  (`SceneComponent.K2_AddLocalRotation` (`self.SM_Kitchen_Cabinet_Hanging_04`) (`KismetMathLibrary.MakeRotator` 0.0 0.0 (`self.Cabinet Open Angle [L]`)) false false)
  (`SceneComponent.K2_AddLocalRotation` (`self.SM_Kitchen_Cabinet_Hanging_02`) (`KismetMathLibrary.MakeRotator` 0.0 0.0 (* (`self.Cabinet Center Open Angle [L]`) -1.0)) false false)
  (`SceneComponent.K2_AddLocalRotation` (`self.SM_Kitchen_Cabinet_Hanging_01`) (`KismetMathLibrary.MakeRotator` 0.0 0.0 (`self.Cabinet Center Open Angle [R]`)) false false)
  (`SceneComponent.K2_AddLocalRotation` (`self.SM_Kitchen_Cabinet_Hanging_03`) (`KismetMathLibrary.MakeRotator` 0.0 0.0 (`self.Cabinet Open Angle [R]`)) false false))