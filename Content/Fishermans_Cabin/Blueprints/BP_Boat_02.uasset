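; BP_Boat_02 is a boat prop for the Fisherman's Cabin environment, with parts that can be posed through variables.
; The Construction Script adds local rotations to separate meshes for engine block lift, engine steering yaw, propeller blade, power lever and back trunk.
; Each part turns on a single axis driven by its own variable, and the event graph holds only disabled stub events, so nothing animates at runtime.
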(fn `UserConstructionScript`
  (`SceneComponent.K2_AddLocalRotation` (`self.SM_Boat_05`) (`KismetMathLibrary.MakeRotator` (`self.Engine Block Lift`)) false false)
  (`SceneComponent.K2_AddLocalRotation` (`self.SM_Boat_06`) (`KismetMathLibrary.MakeRotator` 0.0 0.0 (`self.Engine Rotation`)) false false)
  (`SceneComponent.K2_AddLocalRotation` (`self.SM_Boat_07`) (`KismetMathLibrary.MakeRotator` 0.0 (`self.Blade Rotation`)) false false)
  (`SceneComponent.K2_AddLocalRotation` (`self.SM_Boat_08`) (`KismetMathLibrary.MakeRotator` (`self.Engine Power Lever`)) false false)
  (`SceneComponent.K2_AddLocalRotation` (`self.SM_Boat_04`) (`KismetMathLibrary.MakeRotator` (`self.Back Trunk Angle`)) false false))